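; Steam flamethrower showcase actor that cycles through activation, firing, firing end and shutdown as something enters and leaves its trigger box.
; A FlipFlop on each overlap event alternates states: entries activate or stop firing, exits start firing or deactivate.
; Each state combines skeletal animations, sound cues and particles, with delays and timelines driving emissive and belt-scroll material parameters.
; Clip insert and eject sequences exist but are not wired to any event.
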(event `self.ReceiveBeginPlay`)

(event `self.Box.OnComponentBeginOverlap`
  (params (OverlappedComponent :type "PrimitiveComponent Object Reference") (OtherActor :type "Actor Object Reference") (OtherComp :type "PrimitiveComponent Object Reference") (OtherBodyIndex :type Integer) (bFromSweep :type Boolean) (SweepResult :type "HitResult Structure (by ref)"))
  (bind _steam_flamethrower (`self.Steam_Flamethrower`))
  (bind _belt (`self.Belt`))
  (`/Engine/EditorBlueprintResources/StandardMacros.FlipFlop`
    (:`A`
      ;[1 1 1] Activation
      (`SkeletalMeshComponent.PlayAnimation` _steam_flamethrower "/Game/Steam_Flamethrower/Animation/AS_Activation.AS_Activation" false)
      (`AudioComponent.Play` (`self.Cue_FlameThrower_Activate_Spinup`) 0.0)
      (`AudioComponent.Play` (`self.Cue_FlameThrower_Energy_Spinup`) 0.0)
      (`|ExecutionSequence`
        (:`then_0`
          (`KismetSystemLibrary.Delay` 1.0)
          (`AudioComponent.Play` (`self.Cue_Flamethrower_Plasma_Ignition`) 0.0))
        (:`then_1`
          (`KismetSystemLibrary.Delay` 2.0)
          (`SkeletalMeshComponent.PlayAnimation` _steam_flamethrower "/Game/Steam_Flamethrower/Animation/AS_Idle.AS_Idle" true)
          (`AudioComponent.Play` (`self.Cue_FlameThrower_Gas_Idle`) 0.0)
          (`AudioComponent.Play` (`self.Cue_FlameThrower_Activate_Idle`) 0.0))
        (:`then_2`
          (bind (_direction _emissive_gage_start _emissive_barrel_start) (`Timeline|Emissive_Start` :!via `PlayFromStart`)
            (:`Update`
              (`MeshComponent.SetScalarParameterValueOnMaterials` _steam_flamethrower "Emissive_Power" _emissive_gage_start)
              (`MeshComponent.SetScalarParameterValueOnMaterials` (`self.Barrel`) "Emissive_Power" _emissive_barrel_start)
              (bind (_direction_2 _belt_uv_start) (`Timeline|Belt_UV_Start`)
                (:`Update`
                  (`MeshComponent.SetScalarParameterValueOnMaterials` _belt "U_Offset" _belt_uv_start)
                  (`KismetSystemLibrary.Delay` 2.0)
                  (bind (_direction_3 _belt_uv_idle) (`Timeline|Belt_UV_Idle`)
                    (:`Update`
                      (`MeshComponent.SetScalarParameterValueOnMaterials` _belt "U_Offset" _belt_uv_idle))))))))
        (:`then_3`
          (`KismetSystemLibrary.Delay` 1.16)
          (`ActorComponent.Activate` (`self.PS_Flamethrower_Plasma`) false))))
    (:`B`
      ;[1 1 1] Firing_End
      (`SkeletalMeshComponent.PlayAnimation` (`self.Steam_Flamethrower`) "/Game/Steam_Flamethrower/Animation/AS_Shooting_End.AS_Shooting_End" false)
      (`AudioComponent.Play` (`self.Cue_FlameThrower_Gas_Idle`) 0.0)
      (`AudioComponent.Play` (`self.Cue_FlameThrower_Activate_Idle`) 0.0)
      (`AudioComponent.Play` (`self.Cue_Flamethrower_Shot`) 0.0)
      (`ActorComponent.Activate` (`self.PS_Flamethrower_Plasma`) false)
      (`MeshComponent.SetScalarParameterValueOnMaterials` (`self.Barrel`) "Emissive_Power" 1.0)
      (`MeshComponent.SetScalarParameterValueOnMaterials` (`self.Steam_Flamethrower`) "Emissive_Power" 1.0)
      (`AudioComponent.Stop` (`self.Cue_Flamethrower_Shot`))
      (`ActorComponent.Deactivate` (`self.PS_Flamethrower_Firing_Start`))
      (`KismetSystemLibrary.Delay` 2.0)
      (`SkeletalMeshComponent.PlayAnimation` (`self.Steam_Flamethrower`) "/Game/Steam_Flamethrower/Animation/AS_Idle.AS_Idle" true))))

(event `self.Box.OnComponentEndOverlap`
  (params (OverlappedComponent :type "PrimitiveComponent Object Reference") (OtherActor :type "Actor Object Reference") (OtherComp :type "PrimitiveComponent Object Reference") (OtherBodyIndex :type Integer))
  (bind _steam_flamethrower (`self.Steam_Flamethrower`))
  (`/Engine/EditorBlueprintResources/StandardMacros.FlipFlop`
    (:`A`
      ;[1 1 1] Firing_Start
      (`SkeletalMeshComponent.PlayAnimation` (`self.Steam_Flamethrower`) "/Game/Steam_Flamethrower/Animation/AS_Shooting_Loop_Start.AS_Shooting_Loop_Start" true)
      (`AudioComponent.Play` (`self.Cue_Flamethrower_Shot`) 0.0)
      (`AudioComponent.Play` (`self.Cue_Flamethrower_Shot_Start`) 0.0)
      (`AudioComponent.Play` (`self.Cue_FlameThrower_Gas_Idle`) 0.0)
      (`AudioComponent.Play` (`self.Cue_FlameThrower_Activate_Idle`) 0.0)
      (`ActorComponent.Activate` (`self.PS_Flamethrower_Firing_Start`) false)
      (`MeshComponent.SetScalarParameterValueOnMaterials` (`self.Barrel`) "Emissive_Power" 1.0)
      (`MeshComponent.SetScalarParameterValueOnMaterials` (`self.Steam_Flamethrower`) "Emissive_Power" 1.0)
      (bind (_direction _belt_uv_2x) (`Timeline|Belt_UV_2X`)
        (:`Update`
          (`MeshComponent.SetScalarParameterValueOnMaterials` (`self.Belt`) "U_Offset" _belt_uv_2x))))
    (:`B`
      ;[1 1 1] Deactivation
      (`SkeletalMeshComponent.PlayAnimation` _steam_flamethrower "/Game/Steam_Flamethrower/Animation/AS_Deactivation.AS_Deactivation" false)
      (`AudioComponent.Play` (`self.Cue_FlameThrower_Deactivate_SpinDown`) 0.0)
      (`AudioComponent.Play` (`self.Cue_FlameThrower_Gas_Deactivate`) 0.0)
      (`AudioComponent.Play` (`self.Cue_FlameThrower_Energy_SpinDown`) 0.0)
      (`|ExecutionSequence`
        (:`then_0`
          (`AudioComponent.Stop` (`self.Cue_FlameThrower_Gas_Idle`))
          (`AudioComponent.Stop` (`self.Cue_FlameThrower_Activate_Idle`)))
        (:`then_1`
          (bind (_direction_2 _emissive_gage_end _emissive_barrel_end _belt_uv_end) (`Timeline|Emissive&UV_End` :!via `PlayFromStart`)
            (:`Update`
              (`MeshComponent.SetScalarParameterValueOnMaterials` _steam_flamethrower "Emissive_Power" _emissive_gage_end)
              (`MeshComponent.SetScalarParameterValueOnMaterials` (`self.Barrel`) "Emissive_Power" _emissive_barrel_end)
              (`MeshComponent.SetScalarParameterValueOnMaterials` (`self.Belt`) "U_Offset" _belt_uv_end))))
        (:`then_2`
          (`KismetSystemLibrary.Delay` 2.0)
          (`ActorComponent.Deactivate` (`self.PS_Flamethrower_Plasma`)))))))

(fn `UserConstructionScript`)