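; Showcase actor for the steam flamethrower that plays its fuel clip eject and insert animations as something enters or leaves a trigger box.
; Begin overlap plays the eject animation and sound, then delayed gas particles and hiding of the Fuel_Tank bone.
; End overlap plays the insert, briefly hiding that bone before showing it again.
; Activation, firing and deactivation logic, with timeline-driven emissive and belt UV effects, is present but never runs.
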(event `self.ReceiveBeginPlay`)

(event `self.Box.OnComponentBeginOverlap`
  (params (OverlappedComponent :type "PrimitiveComponent Object Reference") (OtherActor :type "Actor Object Reference") (OtherComp :type "PrimitiveComponent Object Reference") (OtherBodyIndex :type Integer) (bFromSweep :type Boolean) (SweepResult :type "HitResult Structure (by ref)"))
  ;[1 1 1] Clip_Eject
  (`SkeletalMeshComponent.PlayAnimation` (`self.Steam_Flamethrower`) "/Game/Steam_Flamethrower/Animation/AS_Clip_Eject.AS_Clip_Eject" false)
  (`AudioComponent.Play` (`self.Cue_FlameThrower_Clip_Eject`) 0.0)
  (`|ExecutionSequence`
    (:`then_0`
      (`KismetSystemLibrary.Delay` 0.6)
      (`ActorComponent.Activate` (`self.PS_Clip_Gas`) false))
    (:`then_1`
      (`KismetSystemLibrary.Delay` 1.15)
      (`SkinnedMeshComponent.HideBoneByName` (`self.Steam_Flamethrower`) "Fuel_Tank" "PBO_None"))))

(event `self.Box.OnComponentEndOverlap`
  (params (OverlappedComponent :type "PrimitiveComponent Object Reference") (OtherActor :type "Actor Object Reference") (OtherComp :type "PrimitiveComponent Object Reference") (OtherBodyIndex :type Integer))
  ;[1 1 1] Clip_Insert
  (`SkeletalMeshComponent.PlayAnimation` (`self.Steam_Flamethrower`) "/Game/Steam_Flamethrower/Animation/AS_Clip_Insert.AS_Clip_Insert" false)
  (`SkinnedMeshComponent.HideBoneByName` (`self.Steam_Flamethrower`) "Fuel_Tank" "PBO_None")
  (`AudioComponent.Play` (`self.Cue_FlameThrower_Clip_Insert`) 0.0)
  (`KismetSystemLibrary.Delay` 0.1)
  (`SkinnedMeshComponent.UnHideBoneByName` (`self.Steam_Flamethrower`) "Fuel_Tank"))

(fn `UserConstructionScript`)