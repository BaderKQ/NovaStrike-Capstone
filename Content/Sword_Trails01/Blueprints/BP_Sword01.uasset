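; BP_Sword01 is a sword actor that swings with randomized rotation and carries a configurable trail effect, apparently to showcase sword trails.
; An Animation timeline, started on BeginPlay, drives the sword's relative rotation, scaled by a random multiplier per axis.
; A looping timer re-rolls those multipliers every couple of seconds to vary the motion.
; The construction script assigns the FX variable to the NSTrail01 effect component.
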(event `self.ReceiveBeginPlay`
  (`|ExecutionSequence`
    (:`then_0`
      (bind (_direction _x _y _z) (`Timeline|animation` :!via `PlayFromStart`)
        (:`Update`
          (`SceneComponent.K2_SetRelativeRotation` (`self.Sword01`) (`KismetMathLibrary.MakeRotator` (* _x (`self.Random_X`)) (* _y (`self.Random_Y`)) (* _z (`self.Random_Z`))) false false))))
    (:`then_1`
      (`KismetSystemLibrary.K2_SetTimer` null "set_Random_animation" 2.0 true))))

(event `set_Random_animation`
  (set `self.Random_X` (`KismetMathLibrary.RandomFloatInRange` 0.1 1.0))
  (set `self.Random_Y` (`KismetMathLibrary.RandomFloatInRange` 0.1 1.0))
  (set `self.Random_Z` (`KismetMathLibrary.RandomFloatInRange` 0.1 1.0)))

(fn `UserConstructionScript`
  (`NiagaraComponent.SetAsset` (`self.NS_Trail01`) (`self.FX`)))